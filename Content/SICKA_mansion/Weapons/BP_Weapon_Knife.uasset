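; BP_Weapon_Knife is a melee knife weapon whose Fire event performs a short-range attack.
; Fire runs a multi sphere trace forward from the knife along its Arrow's direction, ignoring the player pawn.
; Each hit takes damage, receives a hit reaction message, and spawns an impact particle and cut sound; a miss plays a swing sound.
; In parallel, a brief delay clears the Attacking flag on the player's anim reference.
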(event `/Game/ClassicSurvivalHorrorTemplate/Blueprints/Weapons/BP_WeaponInterface.Fire`
  (bind _returnvalue (`self.K2_GetActorLocation`))
  (`|ExecutionSequence`
    (:`then_0`
      ;[1 1 1] Stop attack after specific time
      (`KismetSystemLibrary.Delay` 0.06)
      (bind _asbp_mixamo_player (cast `/Game/ClassicSurvivalHorrorTemplate/Blueprints/Player/BP_MixamoPlayer` (`GameplayStatics.GetPlayerPawn` 0)))
      (set `/Game/ClassicSurvivalHorrorTemplate/Blueprints/Player/BP_PlayerMixamoAnimBP.Attacking?` false (`/Game/ClassicSurvivalHorrorTemplate/Blueprints/Player/BP_MixamoPlayer.AnimReference` _asbp_mixamo_player)))
    (:`then_1`
      ;[1 1 1] Linetrace
      (bind (_outhits _returnvalue_2) (`KismetSystemLibrary.SphereTraceMulti` _returnvalue (+ _returnvalue (* (`KismetMathLibrary.GetForwardVector` (`SceneComponent.K2_GetComponentRotation` (`self.Arrow`))) 30.0)) 35.0 "TraceTypeQuery1" false (`|MakeArray` (`GameplayStatics.GetPlayerPawn` 0) :!type "Actor Object Reference")))
      (if _returnvalue_2
        (for _array_element _outhits
          (bind (_bblockinghit _binitialoverlap _time _distance _location _impactpoint _normal _impactnormal _physmat _hitactor) (`GameplayStatics.BreakHitResult` _array_element))
          ;[1 1 1] Deal damage
          (`GameplayStatics.ApplyDamage` _hitactor (`self.Damage`))
          ;[1 1 1] Create particle at impact point
          (`GameplayStatics.SpawnEmitterAtLocation` "/Game/ClassicSurvivalHorrorTemplate/Particles/GunFire_Particle.GunFire_Particle" _impactpoint (struct) (0.5 0.5 0.5))
          ;[1 1 1] Make enemy react
          (message `/Game/ClassicSurvivalHorrorTemplate/Blueprints/Enemies/BP_EnemyInterface.HitReaction` _hitactor)
          ;[1 1 1] Cut sound
          (`GameplayStatics.PlaySoundAtLocation` "/Game/ClassicSurvivalHorrorTemplate/Audio/SFX/Cue/KnifeCut_Cue.KnifeCut_Cue" (`self.K2_GetActorLocation`) (struct) 1.0 1.0 0.0 null null null))
        (else
          ;[1 1 1] Swing sound
          (`GameplayStatics.PlaySoundAtLocation` "/Game/ClassicSurvivalHorrorTemplate/Audio/SFX/Cue/MeleeSwing_Cue.MeleeSwing_Cue" (`self.K2_GetActorLocation`) (struct) 1.0 1.0 0.0 null null null))))))

(fn `UserConstructionScript`)