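; BP_Weapon_Shotgun is the shotgun weapon Blueprint, handling what happens when it fires.
; Fire plays the gunshot sound and muzzle particle, then runs a short, thick multi-sphere trace forward from its Arrow on the Visibility channel, ignoring the player pawn.
; Each hit takes damage, spawns an enlarged impact emitter and receives a HitReaction message so enemies can react.
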(event `/Game/ClassicSurvivalHorrorTemplate/Blueprints/Weapons/BP_WeaponInterface.Fire`
  (bind _returnvalue (`SceneComponent.K2_GetComponentLocation` (`self.Arrow`)))
  (`|ExecutionSequence`
    (:`then_0`
      ;[1 1 1] Play Sound
      (`GameplayStatics.PlaySoundAtLocation` "/Game/ClassicSurvivalHorrorTemplate/Audio/SFX/Cue/ShotgunFire_Cue.ShotgunFire_Cue" (`self.K2_GetActorLocation`) (struct) 1.0 1.0 0.0 null null null)
      ;[1 1 1] Activate GunFire Particle
      (`ActorComponent.Activate` (`self.FireParticle`) true))
    (:`then_1`
      ;[1 1 1] Try to find the spot/actor to shoot at
      (bind (_outhits _returnvalue_2) (`KismetSystemLibrary.SphereTraceMulti` _returnvalue (+ _returnvalue (* (`KismetMathLibrary.GetForwardVector` (`SceneComponent.K2_GetComponentRotation` (`self.Arrow`))) 850.0)) 65.0 "TraceTypeQuery1" false (`|MakeArray` (`GameplayStatics.GetPlayerPawn` 0) :!type "Actor Object Reference")))
      (if _returnvalue_2
        (for _array_element _outhits
          (bind (_bblockinghit _binitialoverlap _time _distance _location _impactpoint _normal _impactnormal _physmat _hitactor) (`GameplayStatics.BreakHitResult` _array_element))
          ;[1 1 1] Deal damage
          (`GameplayStatics.ApplyDamage` _hitactor (`self.Damage`))
          ;[1 1 1] Bullet Impact Particle
          (`GameplayStatics.SpawnEmitterAtLocation` "/Game/ClassicSurvivalHorrorTemplate/Particles/GunFire_Particle.GunFire_Particle" _impactpoint (struct) (4.0 4.0 4.0))
          ;[1 1 1] Make enemy react (Message)
          (message `/Game/ClassicSurvivalHorrorTemplate/Blueprints/Enemies/BP_EnemyInterface.HitReaction` _hitactor))))))

(fn `UserConstructionScript`)