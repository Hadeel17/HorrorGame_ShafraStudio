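; Pickup actor for a supply item that the player collects, with a shine effect re-activated every three seconds.
; Box overlap with a Player-tagged actor enables input, and Action either collects directly or opens an optional W_PickupUseQuestion confirmation.
; Next/Previous set Yes/No on that widget, found by class lookup, and a second Action resolves it.
; Collection runs once, passing FSupply to the player, playing a sound, showing a notification and destroying the actor.
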(event `self.ReceiveBeginPlay`
  ;[1 1 1] Event BeginPlay
  ;[1 1 1] Loop (Shining)
  (`ActorComponent.Activate` (`self.Shining`) true :!label _label)
  (`KismetSystemLibrary.Delay` 3.0)
  (goto _label))

(event `InputAction|NextItem`
  (params (Key :type "Key Structure"))
  ;[0 0.02884 0.1406] Action - Pickup
  ;;[0 0 0] Choose Answer
  (:`Pressed`
    (bind _foundwidgets (`WidgetBlueprintLibrary.GetAllWidgetsOfClass` "/Game/ClassicSurvivalHorrorTemplate/UserInterface/W_PickupUseQuestion.W_PickupUseQuestion_C"))
    (if (`KismetArrayLibrary.Array_IsValidIndex` _foundwidgets)
      (for _array_element _foundwidgets
        ;;;[0 0 0] Yes
        (set `/Game/ClassicSurvivalHorrorTemplate/UserInterface/W_PickupUseQuestion.AnswerNoYes` 1 _array_element)))))

(event `InputAction|PreviousItem`
  (params (Key :type "Key Structure"))
  ;[0 0.02884 0.1406] Action - Pickup
  ;;[0 0 0] Choose Answer
  (:`Pressed`
    (bind _foundwidgets (`WidgetBlueprintLibrary.GetAllWidgetsOfClass` "/Game/ClassicSurvivalHorrorTemplate/UserInterface/W_PickupUseQuestion.W_PickupUseQuestion_C"))
    (if (`KismetArrayLibrary.Array_IsValidIndex` _foundwidgets)
      (for _array_element _foundwidgets
        ;;;[0 0 0] No
        (set `/Game/ClassicSurvivalHorrorTemplate/UserInterface/W_PickupUseQuestion.AnswerNoYes` 0 _array_element)))))

(event `self.Box.OnComponentBeginOverlap`
  (params (OverlappedComponent :type "PrimitiveComponent Object Reference") (OtherActor :type "Actor Object Reference") (OtherComp :type "PrimitiveComponent Object Reference") (OtherBodyIndex :type Integer) (bFromSweep :type Boolean) (SweepResult :type "HitResult Structure (by ref)"))
  ;[1 1 1] Overlap Detect
  (if (`self.ActorHasTag` OtherActor "Player")
    (set `self.PlayerActor` OtherActor)
    (`self.EnableInput` (`GameplayStatics.GetPlayerController` 0))))

(event `self.Box.OnComponentEndOverlap`
  (params (OverlappedComponent :type "PrimitiveComponent Object Reference") (OtherActor :type "Actor Object Reference") (OtherComp :type "PrimitiveComponent Object Reference") (OtherBodyIndex :type Integer))
  ;[1 1 1] Overlap Detect
  (if (`self.ActorHasTag` OtherActor "Player")
    (set `self.PlayerActor` null)
    (`self.DisableInput` (`GameplayStatics.GetPlayerController` 0))))

(event `InputAction|Action`
  (params (Key :type "Key Structure"))
  (bind _f_supply_name (break `/Game/ClassicSurvivalHorrorTemplate/Blueprints/Player/S_SupplyInfo` (`self.F_Supply`)))
  ;[0 0.02884 0.1406] Action - Pickup
  (:`Pressed`
    (if (`self.QuestionBeforePickup?`)
      (bind _foundwidgets (`WidgetBlueprintLibrary.GetAllWidgetsOfClass` "/Game/ClassicSurvivalHorrorTemplate/UserInterface/W_PickupUseQuestion.W_PickupUseQuestion_C"))
      (if (`KismetArrayLibrary.Array_IsValidIndex` _foundwidgets)
        (bind _foundwidgets_2 (`WidgetBlueprintLibrary.GetAllWidgetsOfClass` "/Game/ClassicSurvivalHorrorTemplate/UserInterface/W_PickupUseQuestion.W_PickupUseQuestion_C"))
        (for _array_element _foundwidgets_2
          (switch `int` (`/Game/ClassicSurvivalHorrorTemplate/UserInterface/W_PickupUseQuestion.AnswerNoYes` _array_element)
            (:`0`
              ;;[0.000728 0.01042 0] Answer: No
              (bind _foundwidgets_3 (`WidgetBlueprintLibrary.GetAllWidgetsOfClass` "/Game/ClassicSurvivalHorrorTemplate/UserInterface/W_PickupUseQuestion.W_PickupUseQuestion_C"))
              (for _array_element_2 _foundwidgets_3
                (`Widget.RemoveFromParent` _array_element_2)))
            (:`1`
              ;;[0.000728 0.01042 0] Answer: Yes
              (bind _foundwidgets_4 (`WidgetBlueprintLibrary.GetAllWidgetsOfClass` "/Game/ClassicSurvivalHorrorTemplate/UserInterface/W_PickupUseQuestion.W_PickupUseQuestion_C"))
              (for _array_element_3 _foundwidgets_4
                (`Widget.RemoveFromParent` _array_element_3)
                (`/Engine/EditorBlueprintResources/StandardMacros.DoOnce` false :!label _label_2
                  (:`Completed`
                    (message `/Game/ClassicSurvivalHorrorTemplate/Blueprints/Player/PlayerInterface.PickupSupply` (`self.PlayerActor`) (`self.F_Supply`))
                    (`GameplayStatics.PlaySound2D` (`self.PickupSound`) 1.0 1.0 0.0 null null)
                    (`self.ObtainedItemNotification` _f_supply_name " obtained")
                    (`self.K2_DestroyActor`)))))))
        (else
          ;;[0.000728 0.01042 0] Create a question
          (bind _returnvalue (`|CreateWidget` "/Game/ClassicSurvivalHorrorTemplate/UserInterface/W_PickupUseQuestion.W_PickupUseQuestion_C"))
          (`UserWidget.AddToViewport` _returnvalue 0)
          (set `/Game/ClassicSurvivalHorrorTemplate/UserInterface/W_PickupUseQuestion.Question` (`self.TheQuestion`) _returnvalue)))
      (else
        (goto _label_2)))))

(fn `ObtainedItemNotification`
  (params (A :type String) (B :type String) (`Addon(Optional)` :type String))
  (message `/Game/ClassicSurvivalHorrorTemplate/Blueprints/Player/PlayerInterface.Notification` (`self.PlayerActor`) A B `Addon(Optional)`))

(fn `UserConstructionScript`)