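; BP_StoryAdventureGameMode is the game mode that tracks a key-collection objective for the story adventure template.
; On BeginPlay it creates the WB_Tasks HUD widget, sets the starting objective, and counts the BP_MultiKey actors in the level as the required total.
; Its KeyCollected event increments the collected count on the HUD and switches the objective text to "GET OUT!" once every key is found.
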(event `self.ReceiveBeginPlay`
  (`|ExecutionSequence`
    (:`then_0`
      (bind _returnvalue (`|CreateWidget` "/Game/StoryAdvTemplate/Blueprints/UI/WB_Tasks.WB_Tasks_C"))
      (bind _output_get (set `self.HUD` _returnvalue))
      (`UserWidget.AddToViewport` _output_get 0)
      (`TextBlock.SetText` (`/Game/StoryAdvTemplate/Blueprints/UI/WB_Tasks.ObjectiveText` _output_get) "Collect all the keys"))
    (:`then_1`
      (bind _outactors (`GameplayStatics.GetAllActorsOfClass` "/Game/StoryAdvTemplate/Blueprints/Escape/BP_MultiKey.BP_MultiKey_C"))
      (bind _output_get_2 (set `self.NumberOfKeys` (`KismetArrayLibrary.Array_Length` _outactors)))
      (`TextBlock.SetText` (`/Game/StoryAdvTemplate/Blueprints/UI/WB_Tasks.NumberOfKeysText` (`self.HUD`)) (`KismetTextLibrary.Conv_IntToText` _output_get_2)))))

(event `Key Collected`
  (bind _hud (`self.HUD`))
  (bind _result (`/Engine/EditorBlueprintResources/StandardMacros.IncrementInt` (`self.NumberOfKeysCollected`))
    (:`  `
      (`TextBlock.SetText` (`/Game/StoryAdvTemplate/Blueprints/UI/WB_Tasks.NumberOfKeysCollectedText` _hud) (`KismetTextLibrary.Conv_IntToText` _result))
      (if (>= (`self.NumberOfKeysCollected`) (`self.NumberOfKeys`))
        (`TextBlock.SetText` (`/Game/StoryAdvTemplate/Blueprints/UI/WB_Tasks.ObjectiveText` _hud) "GET OUT!")))))

(fn `UserConstructionScript`)