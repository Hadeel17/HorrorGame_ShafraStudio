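; BP_EscapeDoor1 is an escape-level door that the hero opens and closes with Interact while inside its trigger box.
; It stays locked, playing a locked sound, while any BP_MultiKey actor remains in the level.
; Otherwise a FlipFlop alternately plays and reverses a timeline that yaws the mesh, with opening sounds.
; CollectedKeys counts pickups and runs the same interaction check once the required number is reached.
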(event `self.Box.OnComponentBeginOverlap`
  (params (OverlappedComponent :type "PrimitiveComponent Object Reference") (OtherActor :type "Actor Object Reference") (OtherComp :type "PrimitiveComponent Object Reference") (OtherBodyIndex :type Integer) (bFromSweep :type Boolean) (SweepResult :type "HitResult Structure (by ref)"))
  (cast `/Game/StoryAdvTemplate/Blueprints/BP_HeroCharacter` OtherActor)
  (set `self.CanOpen` true))

(event `InputAction|Interact` :consume false
  (params (Key :type "Key Structure"))
  (:`Pressed`
    (if (`self.CanOpen`) :!label _label
      (bind _returnvalue (`GameplayStatics.GetActorOfClass` "/Game/StoryAdvTemplate/Blueprints/Escape/BP_MultiKey.BP_MultiKey_C"))
      (`/Engine/EditorBlueprintResources/StandardMacros.IsValid` _returnvalue
        (:`Is Valid`
          (`AudioComponent.Play` (`self.S_LockedDoor_01`) 0.0)
          (`GameplayStatics.PlaySoundAtLocation` null (0.0 0.0 0.0) (struct) 1.0 1.0 0.0 null null null null))
        (:`Is Not Valid`
          (`/Engine/EditorBlueprintResources/StandardMacros.FlipFlop`
            (:`A`
              (bind (_direction _movemant_) (`Timeline|Timeline` :!label _label_2)
                (:`Update`
                  (`SceneComponent.K2_SetRelativeRotation` (`self.StaticMesh`) (`KismetMathLibrary.MakeRotator` 0.0 0.0 _movemant_) false false)
                  (`AudioComponent.Play` (`self.S_Open_Door_01`) 0.0)
                  (`GameplayStatics.PlaySoundAtLocation` null (0.0 0.0 0.0) (struct) 1.0 1.0 0.0 null null null null))))
            (:`B`
              (goto _label_2 :!via `Reverse`))))))))

(event `self.Box.OnComponentEndOverlap`
  (params (OverlappedComponent :type "PrimitiveComponent Object Reference") (OtherActor :type "Actor Object Reference") (OtherComp :type "PrimitiveComponent Object Reference") (OtherBodyIndex :type Integer))
  (cast `/Game/StoryAdvTemplate/Blueprints/BP_HeroCharacter` OtherActor)
  (set `self.CanOpen` false))

(event `Collected Keys`
  (`/Engine/EditorBlueprintResources/StandardMacros.IncrementInt` (`self.CurrentKeysCollected`)
    (:`  `
      (if (>= (`self.CurrentKeysCollected`) (`self.Numberkeys`))
        (goto _label)))))

(fn `UserConstructionScript`)