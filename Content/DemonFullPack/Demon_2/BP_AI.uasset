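; Demon enemy AI Blueprint that patrols linked PatrolPoints and attacks the hero character.
; PawnSensing moves it toward a seen BP_HeroCharacter within range, otherwise back to its patrol goal.
; On reaching the hero, it plays an attack montage and immediately sphere-traces forward to apply damage, locked until the montage completes.
; A one-shot scream event exists, but its calling graph, like the alternate chase logic, is disconnected.
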(event `self.ReceiveBeginPlay`
  (`self.Patrol`))

(event `Attack Player`
  (bind _attacktracepoint (`self.AttackTracePoint`))
  (bind _returnvalue (`SceneComponent.K2_GetComponentLocation` _attacktracepoint))
  ; Attack Player
  (if (not (`self.Attacking`))
    (set `self.Attacking` true)
    (`|PlayMontage` (`self.Mesh`) "/Game/DemonFullPack/Demon_2/D2_Animations/Anim_Demon2_8_Attack_79_Montage.Anim_Demon2_8_Attack_79_Montage"
      (:`then`
        (bind (_outhit _returnvalue_2) (`KismetSystemLibrary.SphereTraceSingleForObjects` :`Start` _returnvalue :`End` (+ _returnvalue (* (`KismetMathLibrary.GetForwardVector` (`SceneComponent.K2_GetComponentRotation` _attacktracepoint)) 200.0)) :`Radius` 25.0 :`ObjectTypes` (`|MakeArray` "ObjectTypeQuery3" :!type "EObjectTypeQuery Enum") :`DrawDebugType` "ForDuration"))
        (if _returnvalue_2
          (`GameplayStatics.ApplyDamage` (`.HitActor` (`GameplayStatics.BreakHitResult` _outhit)) 10.0)))
      (:`OnCompleted`
        (set `self.Attacking` false)))))

(event `Patrol`
  (bind _goalactor (`self.GoalActor`))
  (bind _goalactor_2 (`self.GoalActor`))
  ; Patrol
  (`/Engine/EditorBlueprintResources/StandardMacros.IsValid` _goalactor :!label _label
    (:`Is Valid`
      (`AITask_MoveTo.AIMoveTo` (`AIBlueprintHelperLibrary.GetAIController` self) (0.0 0.0 0.0) _goalactor
        (:`OnMoveFinished`
          (bind _aspatrol_point (cast `/Game/DemonFullPack/Demon_2/PatrolPoint` _goalactor_2))
          (set `self.previousPoint` _goalactor_2)
          (set `self.GoalActor` (`/Game/DemonFullPack/Demon_2/PatrolPoint.NextPoint` _aspatrol_point))
          (`KismetSystemLibrary.Delay` 1.0)
          (goto _label))))))

(event `Scream At Player`
  ; Scream At Player
  (`/Engine/EditorBlueprintResources/StandardMacros.DoOnce` false :!label _label_2
    (:`Completed`
      (`|PlayMontage` (`self.Mesh`) "/Game/DemonFullPack/Demon_2/D2_Animations/Anim_Demon2_6_IntimidationScream_84_Montage.Anim_Demon2_6_IntimidationScream_84_Montage"
        (:`then`
          (`GameplayStatics.PlaySound2D` "/Game/DemonFullPack/Demon_2/Audio/demonic-roar-40349.demonic-roar-40349" 1.0 1.0 0.0 null null))))))

(event `self.PawnSensing.OnSeePawn`
  (params (Pawn :type "Pawn Object Reference"))
  (bind _asbp_hero_character (cast `/Game/StoryAdvTemplate/Blueprints/BP_HeroCharacter` Pawn))
  (if (< (`KismetMathLibrary.Vector_Distance` (`SceneComponent.K2_GetComponentLocation` (`self.Mesh`)) (`self.K2_GetActorLocation` _asbp_hero_character)) 1000.0)
    (`|AIMoveTo` self (0.0 0.0 0.0) _asbp_hero_character
      (:`OnSuccess`
        (`self.Attack Player`)))
    (else
      (`|AIMoveTo` self (0.0 0.0 0.0) (`self.GoalActor`)
        (:`then`
          (goto _label_2 :!via `Reset`))
        (:`OnSuccess`
          (`self.Patrol`))))))

(fn `UserConstructionScript`)